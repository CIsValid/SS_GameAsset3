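; Idle_Rifle_BP is a damageable actor whose death flags the crew as saved on the player character.
; On BeginPlay it casts player 0 to MyCustomCharacterDevArray and caches the reference.
; AnyDamage subtracts from Health, and at zero or below it sets SavedCrew on that character and destroys itself.
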(event `self.ReceiveBeginPlay`
  (bind _asmy_custom_character_dev_array (cast `/Game/ThirdPersonCPP/MyCustomCharacterDevArray` (`GameplayStatics.GetPlayerCharacter` 0)))
  (set `self.As My Custom Character Dev Array` _asmy_custom_character_dev_array))

(event `self.ReceiveAnyDamage`
  (params (Damage :type "Float (single-precision)") (DamageType :type "DamageType Object Reference") (InstigatedBy :type "Controller Object Reference") (DamageCauser :type "Actor Object Reference"))
  (bind _output_get (set `self.Health` (- (`self.Health`) Damage)))
  (if (<= _output_get 0.0)
    (set `/Game/ThirdPersonCPP/MyCustomCharacterDevArray.bSavedCrew` true (`self.As My Custom Character Dev Array`))
    (`self.K2_DestroyActor`)))

(fn `UserConstructionScript`)