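; Trigger-volume actor that plays an FMOD audio component when something overlaps its Box.
; Begin overlap starts the sound only if it has not yet played and is not already playing, then sets the HasPlayed flag.
; End overlap clears that flag unless PlayOnce is set, allowing either one-shot or repeatable triggers.
; The overlapping actor is not filtered.
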(event `self.Box.OnComponentBeginOverlap`
  (params (OverlappedComponent :type "PrimitiveComponent Object Reference") (OtherActor :type "Actor Object Reference") (OtherComp :type "PrimitiveComponent Object Reference") (OtherBodyIndex :type Integer) (bFromSweep :type Boolean) (SweepResult :type "HitResult Structure (by ref)"))
  (if (not (`self.bHasPlayed?`))
    (bind _returnvalue (`FMODAudioComponent.IsPlaying` (`self.FMODAudio`)))
    (if (not _returnvalue)
      (`FMODAudioComponent.Play` (`self.FMODAudio`))
      (set `self.bHasPlayed?` true))))

(event `self.Box.OnComponentEndOverlap`
  (params (OverlappedComponent :type "PrimitiveComponent Object Reference") (OtherActor :type "Actor Object Reference") (OtherComp :type "PrimitiveComponent Object Reference") (OtherBodyIndex :type Integer))
  (if (not (`self.bPlayOnce?`))
    (set `self.bHasPlayed?` false)))

(fn `UserConstructionScript`)